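; BP_PlayerCharacter is the player character, handling basic axis-driven movement and looking around.
; MoveForward and MoveRight add movement input along the Camera's forward and right vectors, so movement follows the view.
; LookUp and Turn feed controller pitch and yaw, relying on the Camera's pawn rotation setting to turn the view.
; The construction script is empty.
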(event Input|AxisEvents|InputAxisMoveForward
  (params (AxisValue :type Float%20%28single-precision%29))
  ;[1 1 1] Player Movement
  (Pawn|Input|AddMovementInput (Math|Vector|GetForwardVector (Variables|Default|GetCamera)) AxisValue false))

(event Input|AxisEvents|InputAxisMoveRight
  (params (AxisValue :type Float%20%28single-precision%29))
  ;[1 1 1] Player Movement
  (Pawn|Input|AddMovementInput (Math|Vector|GetRightVector (Variables|Default|GetCamera)) AxisValue false))

(event Input|AxisEvents|InputAxisLookUp
  (params (AxisValue :type Float%20%28single-precision%29))
  ;[1 1 1] Looking around
  ;;[1 1 1] To get this to work, we had to change the "Use Pawn Rotation" on the Camera
  (Pawn|Input|AddControllerPitchInput AxisValue))

(event Input|AxisEvents|InputAxisTurn
  (params (AxisValue :type Float%20%28single-precision%29))
  ;[1 1 1] Looking around
  (Pawn|Input|AddControllerYawInput AxisValue))

(fn ConstructionScript)